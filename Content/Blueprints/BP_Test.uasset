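; BP_Test is a test Blueprint that exercises a simple addition function and on-screen debug printing.
; On BeginPlay, AddNumber adds the FiestNumber variable to a constant and the result is printed.
; Tick prints the colored string "현지바보" every frame, while an unreachable self-assignment of the same-named variable also wires into that print.
; The overlap event and construction script are empty.
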(event `self.ReceiveBeginPlay`
  (bind _c (`self.AddNumber` (`self.FiestNumber`) 5))
  (`KismetSystemLibrary.PrintString` (`KismetStringLibrary.Conv_IntToString` _c)))

(event `self.ReceiveTick`
  (params (DeltaSeconds :type "Float (single-precision)"))
  (`KismetSystemLibrary.PrintString` "현지바보" true true (struct :`R` 0.668676 :`G` 0.237802 :`B` 1.0 :`A` 1.0)))

(fn `AddNumber`
  (params (A :type Integer) (B :type Integer))
  (returns (c :type Integer))
  (return (+ A B)))

(fn `UserConstructionScript`)